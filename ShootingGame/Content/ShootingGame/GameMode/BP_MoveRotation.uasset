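; BP_MoveRotation is a shooting-game object whose static mesh spins once activated.
; On BeginPlay it binds to a linked Switch's DoPlay dispatcher, and that event sets the IsPlay flag.
; While the flag is set, Tick adds a fixed relative rotation each frame, so speed depends on frame rate.
; EventOverrap sets the same flag from its argument, allowing the spin to be started or stopped.
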(event `self.ReceiveBeginPlay`
  (add `/Game/ShootingGame/GameMode/BP_Switch.Event_Dispatchers_DoPlay` (`self.Switch`) (`|CreateDelegate` :!event `EventOverrap`)))

(event `self.ReceiveTick`
  (params (DeltaSeconds :type "Float (single-precision)"))
  (if (`self.IsPlay`)
    (`SceneComponent.K2_AddRelativeRotation` (`self.StaticMesh`) (struct :`Yaw` 1.0) false false)))

(event `DoPlay`
  (set `self.IsPlay` true))

(fn `EventOverrap`
  (params (IsBegine :type Boolean))
  (set `self.IsPlay` IsBegine))

(fn `UserConstructionScript`)