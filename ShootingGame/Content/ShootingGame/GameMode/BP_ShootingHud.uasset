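; BP_ShootingHud is the shooting game's HUD Blueprint, showing the local player's health.
; On BeginPlay it creates the ShootingHudWith widget, adds it to the viewport and binds to the first player's BP_ShootingPlayerState.
; If that state is not yet available, a short timer retries the binding.
; HP updates are forwarded to the widget, with an initial push using a hardcoded maximum.
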(event `self.ReceiveBeginPlay`
  (bind _returnvalue (`|CreateWidget` "/Game/ShootingGame/Widget/ShootingHudWith.ShootingHudWith_C"))
  (bind _output_get (set `self.HudWidget` _returnvalue))
  (`UserWidget.AddToViewport` _output_get 0)
  (`self.BindMyPlayerStates`))

(fn `BindMyPlayerStates`
  (bind _asbp_shooting_player_state (cast `/Game/ShootingGame/GameMode/BP_ShootingPlayerState` (`Controller.PlayerState` (`GameplayStatics.GetPlayerController` 0)))
    (:`then`
      (add `/Game/ShootingGame/GameMode/BP_ShootingPlayerState.UpdateHP` _asbp_shooting_player_state (`|CreateDelegate` :!event `EventUpdateHP`))
      (`self.EventUpdateHP` (`/Game/ShootingGame/GameMode/BP_ShootingPlayerState.CurrentHP` _asbp_shooting_player_state) 100.0))
    (:`CastFailed`
      (`KismetSystemLibrary.K2_SetTimer` null "BindMyPlayerStates" 0.01))))

(fn `EventUpdateHP`
  (params (CurrentHP :type "Float (double-precision)") (MaxHP :type "Float (double-precision)"))
  (`/Game/ShootingGame/Widget/ShootingHudWith.SetHP` (`self.HudWidget`) CurrentHP MaxHP))

(fn `UserConstructionScript`)